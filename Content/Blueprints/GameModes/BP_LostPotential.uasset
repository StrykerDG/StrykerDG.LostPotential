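; Game mode for Lost Potential that tracks battery collection and decides how the game ends.
; BeginPlay sets game-only input and counts all BP_Battery actors, and HandleBatteryCollection decrements the remaining count.
; HandleGameEnd broadcasts an invalid-exit notification if batteries remain at the end point; otherwise it halts the player and BP_Dex's depletion timer for a win.
; Win and loss both show the WBP_GameEnding widget with UI-only input.
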(event `InvalidExit`)

(event `self.ReceiveBeginPlay`
  (bind _returnvalue (`GameplayStatics.GetPlayerController` 0))
  (`WidgetBlueprintLibrary.SetInputMode_GameOnly` _returnvalue)
  (`self.EnableInput` _returnvalue)
  (bind _outactors (`GameplayStatics.GetAllActorsOfClass` "/Game/Blueprints/Actors/BP_Battery.BP_Battery_C"))
  (bind _output_get (set `self.TotalBatteries` (`KismetArrayLibrary.Array_Length` _outactors)))
  (set `self.BatteriesRemaining` _output_get))

(fn `HandleBatteryCollection`
  (`/Engine/EditorBlueprintResources/StandardMacros.DecrementInt` (`self.BatteriesRemaining`)))

(fn `HandleEndUI`
  (params (Success :type Boolean))
  (bind _returnvalue (`GameplayStatics.GetPlayerController` 0))
  (set `PlayerController.bShowMouseCursor` true _returnvalue)
  (bind _returnvalue_2 (`|CreateWidget` "/Game/Blueprints/UI/WBP_GameEnding.WBP_GameEnding_C" _returnvalue Success))
  (`UserWidget.AddToViewport` _returnvalue_2 0)
  (`WidgetBlueprintLibrary.SetInputMode_UIOnlyEx` _returnvalue _returnvalue_2 "LockAlways"))

(fn `HandleGameEnd`
  (params (ReachedEnd :type Boolean))
  (bind _returnvalue (`GameplayStatics.GetPlayerCharacter` 0))
  (if ReachedEnd
    (if (> (`self.BatteriesRemaining`) 0)
      (`self.NotifyInvalidExit`)
      (else
        (`self.DisableInput` (`GameplayStatics.GetPlayerController` 0) null)
        (`MovementComponent.StopMovementImmediately` (`Character.CharacterMovement` _returnvalue))
        (bind _asbp_dex (cast `/Game/Blueprints/Characters/BP_Dex` _returnvalue))
        (`KismetSystemLibrary.K2_ClearTimer` _asbp_dex (`/Game/Blueprints/Characters/BP_Dex.DepletionFunction` _asbp_dex))
        (`self.HandleEndUI` true)))
    (else
      (`self.HandleEndUI` false))))

(fn `HandleInvalidExit`
  (`KismetSystemLibrary.PrintString` "Invalid Exit!"))

(fn `UserConstructionScript`)