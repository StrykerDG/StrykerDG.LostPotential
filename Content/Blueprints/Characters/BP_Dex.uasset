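; Player character Dex, with camera-relative movement, zoom and jumping, whose battery level acts as life.
; A looping named timer drains the battery and jumps cost extra, while a one-shot low-energy alarm re-arms on recharge.
; Tick ends the game as a loss through BP_LostPotential at exactly zero battery; the periodic drain, unlike other changes, is unclamped.
; BeginPlay creates the HUD with a reference to Dex.
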(event `InputAxis|CameraZoom`
  (params (AxisValue :type "Float (single-precision)"))
  (bind _output_get (set `self.CurrentZoom` (`KismetMathLibrary.FClamp` (+ (`self.CurrentZoom`) (* AxisValue (`self.ZoomRate`))) (`self.MinZoom`) (`self.MaxZoom`))))
  (set `SpringArmComponent.TargetArmLength` _output_get (`self.SpringArm`)))

(event `InputAxis|MoveForward`
  (params (AxisValue :type "Float (single-precision)"))
  (bind (_returnvalue_roll _returnvalue_pitch _returnvalue_yaw) (`KismetMathLibrary.BreakRotator` (`self.GetControlRotation`)))
  ;[1 1 1] Movement
  (`self.AddMovementInput` (`KismetMathLibrary.GetForwardVector` (`KismetMathLibrary.MakeRotator` 0.0 0.0 _returnvalue_yaw)) AxisValue))

(event `InputAxis|MoveRight`
  (params (AxisValue :type "Float (single-precision)"))
  (bind (_returnvalue_roll _returnvalue_pitch _returnvalue_yaw) (`KismetMathLibrary.BreakRotator` (`self.GetControlRotation`)))
  ;[1 1 1] Movement
  (`self.AddMovementInput` (`KismetMathLibrary.GetRightVector` (`KismetMathLibrary.MakeRotator` 0.0 0.0 _returnvalue_yaw)) AxisValue))

(event `InputAxis|Turn`
  (params (AxisValue :type "Float (single-precision)"))
  ;[1 1 1] Movement
  (`self.AddControllerYawInput` AxisValue))

(event `InputAction|Jump`
  (params (Key :type "Key Structure"))
  ;[1 1 1] Movement
  (:`Pressed`
    (`self.Jump`)
    (`self.DecreaseBatteryLevel` (`self.JumpCost`)))
  (:`Released`
    (`self.StopJumping`)))

(event `InputAxis|LookUp`
  (params (AxisValue :type "Float (single-precision)"))
  ;[1 1 1] Movement
  (`self.AddControllerPitchInput` AxisValue))

(event `self.ReceiveBeginPlay`
  (set `self.BatteryLevel` (`self.InitialBatteryLevel`))
  (set `self.CurrentZoom` (`SpringArmComponent.TargetArmLength` (`self.SpringArm`)))
  (`KismetSystemLibrary.K2_SetTimer` null (`self.DepletionFunction`) (`self.DepletionRate`) true)
  (bind _returnvalue (`|CreateWidget` "/Game/Blueprints/UI/WBP_HUD.WBP_HUD_C" null self))
  (`UserWidget.AddToViewport` _returnvalue 0))

(event `InputAction|Shoot`
  (params (Key :type "Key Structure")))

(event `self.ReceiveTick`
  (params (DeltaSeconds :type "Float (single-precision)"))
  (if (and (== (`self.BatteryLevel`) 0.0) (not (`self.IsDead`)))
    (set `self.IsDead` true)
    (`KismetSystemLibrary.K2_ClearTimer` null (`self.DepletionFunction`))
    (`self.DisableInput` (`GameplayStatics.GetPlayerController` 0))
    (bind _asbp_lost_potential (cast `/Game/Blueprints/GameModes/BP_LostPotential` (`GameplayStatics.GetGameMode`)))
    (`/Game/Blueprints/GameModes/BP_LostPotential.HandleGameEnd` _asbp_lost_potential false)))

(fn `AddBatteryLevel`
  (params (BatteryAmount :type "Float (double-precision)"))
  (set `self.BatteryLevel` (`KismetMathLibrary.FClamp` (+ (`self.BatteryLevel`) BatteryAmount) 0.0 (`self.MaxBatteryLevel`)))
  (`self.ResetAlarm`))

(fn `DecreaseBatteryLevel`
  (params (BatteryAmount :type "Float (double-precision)"))
  (set `self.BatteryLevel` (`KismetMathLibrary.FClamp` (- (`self.BatteryLevel`) BatteryAmount) 0.0 (`self.MaxBatteryLevel`)))
  (`self.SoundAlarm`))

(fn `DecreaseTickingBatteryLevel`
  (set `self.BatteryLevel` (- (`self.BatteryLevel`) (`self.DepletionAmount`)))
  (`self.SoundAlarm`))

(fn `ResetAlarm`
  (if (> (`self.BatteryLevel`) (`self.LowEnergyLevel`))
    (set `self.HasSoundedAlarm` false)))

(fn `SoundAlarm`
  (if (and (<= (`self.BatteryLevel`) (`self.LowEnergyLevel`)) (not (`self.HasSoundedAlarm`)))
    (`GameplayStatics.PlaySoundAtLocation` "/Game/Assets/Audio/Effects/LowEnergy.LowEnergy" (`self.K2_GetActorLocation`) (struct) 1.0 1.0 0.0 null null null)
    (set `self.HasSoundedAlarm` true)))

(fn `UserConstructionScript`)